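; Gameplay ability for hip firing the equipped weapon, repeating shots at the weapon's fire rate.
; Activation, triggered from an event, plays the weapon's attack montage, fires immediately and starts a looping shot timer.
; Each shot traces from weapon to focus, plays weapon effects and applies the weapon's effect spec to any hit actor's ability system.
; The attack-ended gameplay event or montage finishing ends the ability, which clears the timer.
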(event `self.K2_ActivateAbilityFromEvent`
  (params (EventData :type "GameplayEventData Structure (by ref)"))
  (bind _returnvalue (`self.GetEquippedWeaponStaticData`))
  (`AbilityTask_PlayMontageAndWait.CreatePlayMontageAndWaitProxy` "None" (`StaticWeaponData.AttackMontage` _returnvalue)
    (:`then`
      (bind _returnvalue_2 (`KismetSystemLibrary.K2_SetTimerDelegate` (delegate `Shoot`) (/ 1.0 (`StaticWeaponData.FireRate` _returnvalue)) true))
      (set `self.Shoot Timer Handle` _returnvalue_2)
      (`self.Shoot`)
      (`AbilityTask_WaitGameplayEvent.WaitGameplayEvent` (struct :`TagName` "Event.Combat.Attack.Ended") null
        (:`EventReceived`
          (`self.K2_EndAbility`))))
    (:`OnCompleted`
      (`self.K2_EndAbility` :!label _label))
    (:`OnBlendOut`
      (goto _label))
    (:`OnInterrupted`
      (goto _label))
    (:`OnCancelled`
      (goto _label))))

(event `Shoot`
  (bind (_outhitresult _returnvalue) (`self.GetWeaponToFocusTraceResult` (`self.ShootingDistance`) "TraceTypeQuery3"))
  (bind _returnvalue_2 (`AbilitySystemBlueprintLibrary.GetAbilitySystemComponent` (`.HitActor` (`GameplayStatics.BreakHitResult` _outhitresult))))
  (`WeaponActor.PlayWeaponEffects` (`self.GetEquippedWeaponItemActor`) _outhitresult)
  (if _returnvalue
    (`/Engine/EditorBlueprintResources/StandardMacros.IsValid` _returnvalue_2
      (:`Is Valid`
        (`AbilitySystemComponent.BP_ApplyGameplayEffectSpecToSelf` _returnvalue_2 (`self.GetWeaponEffectSpec` _outhitresult))))))

(event `self.K2_OnEndAbility`
  (params (bWasCancelled :type Boolean))
  (`KismetSystemLibrary.K2_ClearAndInvalidateTimerHandle` (`self.Shoot Timer Handle`)))