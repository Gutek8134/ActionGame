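; BP_GA_Aim is a Gameplay Ability that applies an aim camera modifier to the player's camera while aiming.
; On activation it adds the modifier to the PlayerCameraManager and stores the returned instance, ending immediately if the controller or camera manager is invalid.
; It then waits for the Event.Combat.Aim.Ended gameplay event to end itself, and OnEndAbility removes the stored modifier.
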(event `self.K2_ActivateAbility`
  (bind (_owneractor _avataractor _playercontroller) (break `GameplayAbilityActorInfo` (`self.GetActorInfo`)))
  (bind _playercameramanager (`PlayerController.PlayerCameraManager` _playercontroller))
  (`/Engine/EditorBlueprintResources/StandardMacros.IsValid` _playercontroller
    (:`Is Valid`
      (`/Engine/EditorBlueprintResources/StandardMacros.IsValid` _playercameramanager
        (:`Is Valid`
          (bind _returnvalue (`PlayerCameraManager.AddNewCameraModifier` _playercameramanager "/Game/CameraModifiers/AimCameraModifier.AimCameraModifier_C"))
          (set `self.Aim Camera Mod Handle` _returnvalue)
          (`AbilityTask_WaitGameplayEvent.WaitGameplayEvent` (struct :`TagName` "Event.Combat.Aim.Ended") null
            (:`EventReceived`
              _)))
        (:`Is Not Valid`
          _)))
    (:`Is Not Valid`
      _))
  (`self.K2_EndAbility`))

(event `self.K2_OnEndAbility`
  (params (bWasCancelled :type Boolean))
  (bind (_owneractor _avataractor _playercontroller) (break `GameplayAbilityActorInfo` (`self.GetActorInfo`)))
  (bind _playercameramanager (`PlayerController.PlayerCameraManager` _playercontroller))
  (`/Engine/EditorBlueprintResources/StandardMacros.IsValid` _playercontroller
    (:`Is Valid`
      (`/Engine/EditorBlueprintResources/StandardMacros.IsValid` _playercameramanager
        (:`Is Valid`
          (`PlayerCameraManager.RemoveCameraModifier` _playercameramanager (`self.Aim Camera Mod Handle`)))))))